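; BP_WorldGenerator builds the game world at BeginPlay as a square grid of BP_WorldChunk actors centered on chunk coordinate zero.
; FGenerateWorld queues every chunk coordinate within the render distance, then starts EGenerateNextChunk.
; That event spawns a chunk at its scaled position, passes coordinates and sizes, and calls its FGenerateChunk.
; It re-arms itself with a near-zero timer, spreading generation over time instead of one blocking loop.
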(event Custom|EGenerateNextChunk
  (if (< (Variables|Default|GetCurrentPendingChunkIndex) (Utilities|Array|Length (Variables|Default|GetPendingChunkCoordinates)))
    (Variables|Default|SetCurrentChunkCoordinate (Utilities|Array|Get(acopy) (Variables|Default|GetPendingChunkCoordinates) (Variables|Default|GetCurrentPendingChunkIndex)))
    (bind _returnvalue (Game|SpawnActorfromClass "/Game/Blueprints/World/BP_WorldChunk.BP_WorldChunk_C" (Math|Transform|MakeTransform (Math|Vector|MakeVector (* (.x (Variables|Default|GetCurrentChunkCoordinate)) (Variables|Default|GetChunkSize) (Variables|Default|GetTileSize)) (* (.y (Variables|Default|GetCurrentChunkCoordinate)) (Variables|Default|GetChunkSize) (Variables|Default|GetTileSize)) 0.0) "0, 0, 0" "1.000000,1.000000,1.000000") "Undefined" "MultiplyWithRoot" 0 0))
    (bind _output_get (Variables|Default|SetSpawnedChunkReference _returnvalue))
    (Variables|/Game/Blueprints/World/BP_WorldChunk.BP_WorldChunk_C|SetChunkCoordinateX _output_get (Math|Float|Truncate (.x (Variables|Default|GetCurrentChunkCoordinate))))
    (Variables|/Game/Blueprints/World/BP_WorldChunk.BP_WorldChunk_C|SetChunkCoordinateY (Variables|Default|GetSpawnedChunkReference) (Math|Float|Truncate (.y (Variables|Default|GetCurrentChunkCoordinate))))
    (Variables|/Game/Blueprints/World/BP_WorldChunk.BP_WorldChunk_C|SetChunkSize (Variables|Default|GetSpawnedChunkReference) (Variables|Default|GetChunkSize))
    (Variables|/Game/Blueprints/World/BP_WorldChunk.BP_WorldChunk_C|SetTileSize (Variables|Default|GetSpawnedChunkReference) (Variables|Default|GetTileSize))
    (Default|FGenerateChunk (Variables|Default|GetSpawnedChunkReference))
    (Math|Integer|IncrementInt (Variables|Default|GetCurrentPendingChunkIndex)
      (:%20%20
        (Utilities|Time|SetTimerbyEvent (delegate Custom|EGenerateNextChunk) 0.0001)))))

(event EventBeginPlay
  (CallFunction|FGenerateWorld))

(fn ConstructionScript)

(fn FGenerateWorld
  (bind _renderdistanceinchunks (Variables|Default|GetRenderDistanceInChunks))
  (bind _renderdistanceinchunks_2 (Variables|Default|GetRenderDistanceInChunks))
  (for _index (range (* _renderdistanceinchunks_2 -1) _renderdistanceinchunks_2)
    (LocalVariables|SetChunkY _index)
    (for _index_2 (range (* _renderdistanceinchunks -1) _renderdistanceinchunks)
      (bind _output_get (LocalVariables|SetChunkX _index_2))
      (Utilities|Array|Add (Variables|Default|GetPendingChunkCoordinates) (Math|Vector2D|MakeVector2D (Math|Conversions|ToFloat(Integer) _output_get) (Math|Conversions|ToFloat(Integer) (LocalVariables|GetChunkY))))))
  (Variables|Default|SetCurrentPendingChunkIndex 0)
  (CallFunction|EGenerateNextChunk))