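; BP_WorldGeneratorOLD builds a square grid of world chunks around coordinate origin when play begins.
; FGenerateWorld queues every chunk coordinate within the render distance from GenerationSettings.
; EGenerateNextChunk spawns a BP_WorldChunkOLD at the scaled position, passes it its coordinate and settings, then calls its FGenerateChunk.
; The event re-arms itself with a near-zero timer, staggering generation one chunk per call instead of one blocking loop.
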(event Custom|EGenerateNextChunk
  (if (< (Variables|Default|GetCurrentPendingChunkIndex) (Utilities|Array|Length (Variables|Default|GetPendingChunkCoordinates)))
    (Variables|Default|SetCurrentChunkCoordinate (Utilities|Array|Get(acopy) (Variables|Default|GetPendingChunkCoordinates) (Variables|Default|GetCurrentPendingChunkIndex)))
    (bind _returnvalue (Game|SpawnActorfromClass "/Game/Blueprints/World/BP_WorldChunkOLD.BP_WorldChunkOLD_C" (Math|Transform|MakeTransform (Math|Vector|MakeVector (* (.x (Variables|Default|GetCurrentChunkCoordinate)) (.ChunkSize (Utilities|Struct|BreakF_GenerationSettings (Variables|Default|GetGenerationSettings))) (.TileSize (Utilities|Struct|BreakF_GenerationSettings (Variables|Default|GetGenerationSettings)))) (* (.y (Variables|Default|GetCurrentChunkCoordinate)) (.ChunkSize (Utilities|Struct|BreakF_GenerationSettings (Variables|Default|GetGenerationSettings))) (.TileSize (Utilities|Struct|BreakF_GenerationSettings (Variables|Default|GetGenerationSettings)))) 0.0) "0, 0, 0" "1.000000,1.000000,1.000000") "Undefined" "MultiplyWithRoot" 0 0))
    (bind _output_get (Variables|Default|SetSpawnedChunkReference _returnvalue))
    (Variables|/Game/Blueprints/World/BP_WorldChunkOLD.BP_WorldChunkOLD_C|SetChunkCoordinateX _output_get (Math|Float|Truncate (.x (Variables|Default|GetCurrentChunkCoordinate))))
    (Variables|/Game/Blueprints/World/BP_WorldChunkOLD.BP_WorldChunkOLD_C|SetChunkCoordinateY (Variables|Default|GetSpawnedChunkReference) (Math|Float|Truncate (.y (Variables|Default|GetCurrentChunkCoordinate))))
    (Variables|/Game/Blueprints/World/BP_WorldChunkOLD.BP_WorldChunkOLD_C|SetGenerationSettings (Variables|Default|GetSpawnedChunkReference) (Variables|Default|GetGenerationSettings))
    (Default|FGenerateChunk (Variables|Default|GetSpawnedChunkReference))
    (Math|Integer|IncrementInt (Variables|Default|GetCurrentPendingChunkIndex)
      (:%20%20
        (Utilities|Time|SetTimerbyEvent (delegate Custom|EGenerateNextChunk) 0.0001)))))

(event EventBeginPlay
  (CallFunction|FGenerateWorld))

(fn ConstructionScript)

(fn FGenerateWorld
  (bind _generationsettings (Variables|Default|GetGenerationSettings))
  (bind _renderdistance (Utilities|Struct|BreakF_GenerationSettings _generationsettings))
  (for _index (range (* _renderdistance -1) _renderdistance)
    (LocalVariables|SetChunkY _index)
    (for _index_2 (range (* _renderdistance -1) _renderdistance)
      (bind _output_get (LocalVariables|SetChunkX _index_2))
      (Utilities|Array|Add (Variables|Default|GetPendingChunkCoordinates) (Math|Vector2D|MakeVector2D (Math|Conversions|ToFloat(Integer) _output_get) (Math|Conversions|ToFloat(Integer) (LocalVariables|GetChunkY))))))
  (Variables|Default|SetCurrentPendingChunkIndex 0)
  (CallFunction|EGenerateNextChunk))