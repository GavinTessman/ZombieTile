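; World generation function library that classifies a coordinate's region (by land cutoff), temperature and moisture from Perlin noise.
; Each sample's offset comes from a random stream seeded with world seed and layer ID, though several calls omit the seed.
; Region sums four octaves against a cutoff shifted by a huge layer, yielding normalized elevation.
; Temperature and moisture pick the strongest two-scale noise, with hot and cold settings cross-wired.
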(fn FGetNoiseatCoordinate
  (params (X :type Integer) (Y :type Integer) (Scale :type Float%20%28double-precision%29) (WorldSeed :type Integer) (NoiseID :type Integer))
  ;[0.15 0.15 0.15 0.5 14] Build Noise Seed
  (bind _returnvalue (Class|NoiseBlueprintLibrary|HashCombineFastInt WorldSeed NoiseID))
  (bind _output_get (LocalVariables|SetRandomStream (Math|Random|MakeRandomStream _returnvalue)))
  ;[0.15 0.15 0.15 0.5] Generate Seed Offsets
  (LocalVariables|SetOffsetX (Math|Random|RandomFloatinRangefromStream _output_get -1e+05 1e+05))
  (LocalVariables|SetOffsetY (Math|Random|RandomFloatinRangefromStream (LocalVariables|GetRandomStream) -1e+05 1e+05))
  ;[0.15 0.15 0.15 0.5] Sample Perlin Noise
  (bind _returnvalue_2 (Class|NoiseBlueprintLibrary|GetPerlinNoise2D (Math|Vector2D|MakeVector2D (/ (+ (Math|Conversions|ToFloat(Integer) X) (LocalVariables|GetOffsetX)) Scale) (/ (+ (Math|Conversions|ToFloat(Integer) Y) (LocalVariables|GetOffsetY)) Scale))))
  (return _returnvalue_2))

(fn FGetDoubleNoiseatCoordinate
  (params (X :type Integer) (Y :type Integer) (SmallScale :type Float%20%28double-precision%29) (LargeScale :type Float%20%28double-precision%29) (SmallWeight :type Float%20%28double-precision%29) (LargeWeight :type Float%20%28double-precision%29) (WorldSeed :type Integer) (NoiseID :type Integer))
  ;[0.15 0.15 0.15 0.5] Sample Large Noise
  (LocalVariables|SetLargeNoise (WorldGeneration|Utility|FGetNoiseatCoordinate X Y LargeScale WorldSeed NoiseID))
  ;[0.15 0.15 0.15 0.5] Sample Small Noise
  (LocalVariables|SetSmallNoise (WorldGeneration|Utility|FGetNoiseatCoordinate X Y SmallScale WorldSeed NoiseID))
  ;[0.15 0.15 0.15 0.5] Combine Noise Layers
  (bind _output_get (LocalVariables|SetFinalNoise (+ (* (LocalVariables|GetLargeNoise) LargeWeight) (* (LocalVariables|GetSmallNoise) SmallWeight))))
  (return _output_get))

(fn FGetRegionContextatCoordinate
  (params (X :type Integer) (Y :type Integer) (RegionNoiseSettings :type F%20Region%20Noise%20Settings%20Structure) (WorldSeed :type Integer))
  (bind (_noisevalue _hugenoiseoutput) (WorldGeneration|Region|FGetRegionNoiseatCoordinate X Y RegionNoiseSettings WorldSeed))
  ;[0.15 0.15 0.15 0.5] Sample Region Noise
  (LocalVariables|SetRegionNoise _noisevalue)
  ;[0.15 0.15 0.15 0.5] Determine Land Cutoff
  (LocalVariables|SetLandCutoff (+ _hugenoiseoutput (Utilities|Struct|BreakF_RegionNoiseSettings RegionNoiseSettings)))
  ;[0.15 0.15 0.15 0.5] Determine Region Type
  (if (<= (LocalVariables|GetRegionNoise) (LocalVariables|GetLandCutoff))
    (return (Utilities|Struct|MakeF_RegionContext "NewEnumerator1" (/ (- (LocalVariables|GetRegionNoise) (LocalVariables|GetLandCutoff)) (- 1.0 (LocalVariables|GetLandCutoff)))))
    (else
      (return (Utilities|Struct|MakeF_RegionContext "NewEnumerator0" (/ (- (LocalVariables|GetRegionNoise) (LocalVariables|GetLandCutoff)) (- 1.0 (LocalVariables|GetLandCutoff))))))))

(fn FGetRegionNoiseatCoordinate
  (params (X :type Integer) (Y :type Integer) (RegionNoiseSettings :type F%20Region%20Noise%20Settings%20Structure) (WorldSeed :type Integer))
  (bind (_hugenoiselayersettings _largenoiselayersettings _mediumnoiselayersettings _smallnoiselayersettings _tinynoiselayersettings) (Utilities|Struct|BreakF_RegionNoiseSettings RegionNoiseSettings))
  (bind (_largenoiselayersettings_2 _mediumnoiselayersettings_2 _smallnoiselayersettings_2 _tinynoiselayersettings_2) (Utilities|Struct|BreakF_RegionNoiseSettings RegionNoiseSettings))
  (bind (_maxscale _layerid) (Utilities|Struct|BreakF_NoiseLayerSettings _hugenoiselayersettings))
  (bind (_maxscale_2 _layerid_2) (Utilities|Struct|BreakF_NoiseLayerSettings _tinynoiselayersettings))
  (bind (_maxscale_3 _layerid_3) (Utilities|Struct|BreakF_NoiseLayerSettings _largenoiselayersettings))
  (bind (_maxscale_4 _layerid_4) (Utilities|Struct|BreakF_NoiseLayerSettings _mediumnoiselayersettings))
  (bind (_maxscale_5 _layerid_5) (Utilities|Struct|BreakF_NoiseLayerSettings _smallnoiselayersettings))
  ;[0.15 0.15 0.15 0.5] Set Region Noise Values
  (LocalVariables|SetHugeNoise (WorldGeneration|Utility|FGetNoiseatCoordinate X Y _maxscale WorldSeed _layerid))
  (LocalVariables|SetLargeNoise (WorldGeneration|Utility|FGetNoiseatCoordinate X Y _maxscale_3 0 _layerid_3))
  (LocalVariables|SetMediumNoise (WorldGeneration|Utility|FGetNoiseatCoordinate X Y _maxscale_4 0 _layerid_4))
  (LocalVariables|SetSmallNoise (WorldGeneration|Utility|FGetNoiseatCoordinate X Y _maxscale_5 0 _layerid_5))
  (LocalVariables|SetTinyNoise (WorldGeneration|Utility|FGetNoiseatCoordinate X Y _maxscale_2 0 _layerid_2))
  ;[0.15 0.15 0.15 0.5] Calculate FinalRegionNoise
  (LocalVariables|SetFinalRegionNoise (+ (* (LocalVariables|GetLargeNoise) (Utilities|Struct|BreakF_NoiseLayerSettings _largenoiselayersettings_2)) (* (LocalVariables|GetMediumNoise) (Utilities|Struct|BreakF_NoiseLayerSettings _mediumnoiselayersettings_2)) (* (LocalVariables|GetSmallNoise) (Utilities|Struct|BreakF_NoiseLayerSettings _smallnoiselayersettings_2)) (* (LocalVariables|GetTinyNoise) (Utilities|Struct|BreakF_NoiseLayerSettings _tinynoiselayersettings_2))))
  (return (LocalVariables|GetFinalRegionNoise) (* (LocalVariables|GetHugeNoise) (Utilities|Struct|BreakF_NoiseLayerSettings (Utilities|Struct|BreakF_RegionNoiseSettings RegionNoiseSettings)))))

(fn FGetTemperatureContextatCoordinate
  (params (X :type Integer) (Y :type Integer) (TemperatureNoiseSettings :type F%20Temperature%20Noise%20Settings%20Structure) (WorldSeed :type Integer))
  (bind (_hotnoiselayersettings _temperatenoiselayersettings _coldnoiselayersettings) (Utilities|Struct|BreakF_TemperatureNoiseSettings TemperatureNoiseSettings))
  (bind (_minscale _maxscale _minweight _maxweight _layerid) (Utilities|Struct|BreakF_NoiseLayerSettings _hotnoiselayersettings))
  (bind (_minscale_2 _maxscale_2 _minweight_2 _maxweight_2 _layerid_2) (Utilities|Struct|BreakF_NoiseLayerSettings _temperatenoiselayersettings))
  (bind (_minscale_3 _maxscale_3 _minweight_3 _maxweight_3 _layerid_3) (Utilities|Struct|BreakF_NoiseLayerSettings _coldnoiselayersettings))
  ;[0.15 0.15 0.15 0.5] Determine Temperature Noise Values
  (LocalVariables|SetColdNoise (WorldGeneration|Utility|FGetDoubleNoiseatCoordinate X Y _minscale _maxscale _minweight _maxweight WorldSeed _layerid))
  (LocalVariables|SetTemperateNoise (WorldGeneration|Utility|FGetDoubleNoiseatCoordinate X Y _minscale_2 _maxscale_2 _minweight_2 _maxweight_2 WorldSeed _layerid_2))
  (LocalVariables|SetHotNoise (WorldGeneration|Utility|FGetDoubleNoiseatCoordinate X Y _minscale_3 _maxscale_3 _minweight_3 _maxweight_3 0 _layerid_3))
  ;[0.15 0.15 0.15 0.5] Determine Temperature Type
  (if (and (> (LocalVariables|GetColdNoise) (LocalVariables|GetTemperateNoise)) (> (LocalVariables|GetColdNoise) (LocalVariables|GetHotNoise)))
    (LocalVariables|SetTemperatureType "NewEnumerator2")
    (elif (and (> (LocalVariables|GetTemperateNoise) (LocalVariables|GetColdNoise)) (> (LocalVariables|GetTemperateNoise) (LocalVariables|GetHotNoise)))
      (LocalVariables|SetTemperatureType "NewEnumerator1")
      (else
        (LocalVariables|SetTemperatureType "NewEnumerator0"))))
  (return (Utilities|Struct|MakeF_TemperatureContext (LocalVariables|GetTemperatureType) (LocalVariables|GetHotNoise) (LocalVariables|GetTemperateNoise) (LocalVariables|GetColdNoise))))

(fn FGetMoistureContextatCoordinate
  (params (X :type Integer) (Y :type Integer) (MoistureNoiseSettings :type F%20Moisture%20Noise%20Settings%20Structure) (WorldSeed :type Integer))
  (bind (_drynoiselayersettings _wetnoiselayersettings) (Utilities|Struct|BreakF_MoistureNoiseSettings MoistureNoiseSettings))
  (bind (_minscale _maxscale _minweight _maxweight _layerid) (Utilities|Struct|BreakF_NoiseLayerSettings _drynoiselayersettings))
  (bind (_minscale_2 _maxscale_2 _minweight_2 _maxweight_2 _layerid_2) (Utilities|Struct|BreakF_NoiseLayerSettings _wetnoiselayersettings))
  ;[0.15 0.15 0.15 0.5] Determine Moisture Noise Values
  (LocalVariables|SetDryNoise (WorldGeneration|Utility|FGetDoubleNoiseatCoordinate X Y _minscale _maxscale _minweight _maxweight WorldSeed _layerid))
  (LocalVariables|SetWetNoise (WorldGeneration|Utility|FGetDoubleNoiseatCoordinate X Y _minscale_2 _maxscale_2 _minweight_2 _maxweight_2 WorldSeed _layerid_2))
  ;[0.15 0.15 0.15 0.5] Determine Moisture Type
  (if (< (LocalVariables|GetWetNoise) (LocalVariables|GetDryNoise))
    (LocalVariables|SetMoistureType "NewEnumerator0")
    (else
      (LocalVariables|SetMoistureType "NewEnumerator1")))
  (return (Utilities|Struct|MakeF_MoistureContext (LocalVariables|GetMoistureType) (LocalVariables|GetDryNoise) (LocalVariables|GetWetNoise))))