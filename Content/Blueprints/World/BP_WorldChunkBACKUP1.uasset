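; World chunk backup that holds logic to build a tile grid coloured by WorldDebugView, but the generation body is disconnected and never runs.
; That body fills ISMTiles with instances, passing RGB as custom data.
; Weighted multi-octave Perlin noise splits land from sea against a threshold shifted by huge-scale noise.
; Temperature compares cold, temperate and hot noise with border detail, but all three sample identically, so it always returns Hot.
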(fn ConstructionScript)

(fn FGenerateChunk)

(fn FGetRegionTypeatCoordinate
  (params (X :type Integer) (Y :type Integer))
  (bind (_noisevalue _hugenoiseoutput) (CallFunction|FGetRegionNoiseatCoordinate X Y))
  (if (<= _noisevalue (+ (Variables|Default|GetLandThreshold) (* _hugenoiseoutput (Variables|Default|GetHugeRegionStrength))))
    (return "NewEnumerator1")
    (else
      (return "NewEnumerator0"))))

(fn FGetRegionNoiseatCoordinate
  (params (X :type Integer) (Y :type Integer))
  (bind _largeregionscaledivisor (Variables|Default|GetLargeRegionScaleDivisor))
  (bind _smallregionscaledivisor (Variables|Default|GetSmallRegionScaleDivisor))
  (bind _mediumregionscaledivisor (Variables|Default|GetMediumRegionScaleDivisor))
  (bind _hugeregionscaledivisor (Variables|Default|GetHugeRegionScaleDivisor))
  (LocalVariables|SetLocalX (Math|Conversions|ToFloat(Integer) X))
  (LocalVariables|SetLocalY (Math|Conversions|ToFloat(Integer) Y))
  (bind _returnvalue (Class|NoiseBlueprintLibrary|GetPerlinNoise2D (Math|Vector2D|MakeVector2D (/ (LocalVariables|GetLocalX) _hugeregionscaledivisor) (/ (LocalVariables|GetLocalY) _hugeregionscaledivisor))))
  (LocalVariables|SetHugeNoise _returnvalue)
  (bind _returnvalue_2 (Class|NoiseBlueprintLibrary|GetPerlinNoise2D (Math|Vector2D|MakeVector2D (/ (LocalVariables|GetLocalX) _largeregionscaledivisor) (/ (LocalVariables|GetLocalY) _largeregionscaledivisor))))
  (LocalVariables|SetLargeNoise _returnvalue_2)
  (bind _returnvalue_3 (Class|NoiseBlueprintLibrary|GetPerlinNoise2D (Math|Vector2D|MakeVector2D (/ (LocalVariables|GetLocalX) _mediumregionscaledivisor) (/ (LocalVariables|GetLocalY) _mediumregionscaledivisor))))
  (LocalVariables|SetMediumNoise _returnvalue_3)
  (bind _returnvalue_4 (Class|NoiseBlueprintLibrary|GetPerlinNoise2D (Math|Vector2D|MakeVector2D (/ (LocalVariables|GetLocalX) _smallregionscaledivisor) (/ (LocalVariables|GetLocalY) _smallregionscaledivisor))))
  (LocalVariables|SetSmallNoise _returnvalue_4)
  (bind _returnvalue_5 (Class|NoiseBlueprintLibrary|GetPerlinNoise2D (Math|Vector2D|MakeVector2D (/ (LocalVariables|GetLocalX) 5.0) (/ (LocalVariables|GetLocalY) (Variables|Default|GetTinyRegionScaleDivisor)))))
  (LocalVariables|SetTinyNoise _returnvalue_5)
  (bind _output_get (LocalVariables|SetFinalRegionNoise (+ (* (LocalVariables|GetLargeNoise) (Variables|Default|GetLargeRegionWeight)) (* (LocalVariables|GetMediumNoise) (Variables|Default|GetMediumRegionWeight)) (* (LocalVariables|GetSmallNoise) (Variables|Default|GetSmallRegionWeight)) (* (LocalVariables|GetTinyNoise) (Variables|Default|GetTinyRegionWeight)))))
  (return _output_get (LocalVariables|GetHugeNoise)))

(fn FGetRegionColor
  (params (RegionType :type E_RegionType%20Enum :default "NewEnumerator0") (TemperatureType :type E_TemperatureType%20Enum :default "NewEnumerator0"))
  (switch Utilities|FlowControl|Switch|SwitchonE_WorldDebugView (Variables|Default|GetWorldDebugView)
    (:NewEnumerator0
      (switch Utilities|FlowControl|Switch|SwitchonE_RegionType RegionType
        (:NewEnumerator0
          (return "(R=0.000000,G=1.000000,B=0.000000,A=1.000000)"))
        (:NewEnumerator1
          (return "(R=0.000000,G=0.000000,B=1.000000,A=1.000000)"))))
    (:NewEnumerator1
      (switch Utilities|FlowControl|Switch|SwitchonE_RegionType RegionType
        (:NewEnumerator0
          (switch Utilities|FlowControl|Switch|SwitchonE_TemperatureType TemperatureType
            (:NewEnumerator0
              (return "(R=1.000000,G=0.000000,B=0.000000,A=1.000000)"))
            (:NewEnumerator1
              (return "(R=0.000000,G=1.000000,B=0.000000,A=1.000000)"))
            (:NewEnumerator2
              (return "(R=0.000000,G=0.000000,B=1.000000,A=1.000000)"))))
        (:NewEnumerator1
          (switch Utilities|FlowControl|Switch|SwitchonE_TemperatureType TemperatureType
            (:NewEnumerator0
              (return "(R=1.000000,G=0.000000,B=0.200000,A=1.000000)"))
            (:NewEnumerator1
              (return "(R=0.000000,G=1.000000,B=0.200000,A=1.000000)"))
            (:NewEnumerator2
              (return "(R=0.100000,G=0.100000,B=1.000000,A=1.000000)"))))))
    (:NewEnumerator2
      (return "(R=0.000000,G=0.000000,B=1.000000,A=1.000000)"))
    (:NewEnumerator3
      (return "(R=0.000000,G=1.000000,B=0.000000,A=1.000000)"))))

(fn FGetTemperatureTypeatCoordinate
  (params (X :type Integer) (Y :type Integer))
  (LocalVariables|SetLocalX (Math|Conversions|ToFloat(Integer) X))
  (LocalVariables|SetLocalY (Math|Conversions|ToFloat(Integer) Y))
  (bind (_smallnoiseoutput _largenoiseoutput) (CallFunction|FGetTemperatureNoiseatCoordinate (+ (LocalVariables|GetLocalX) 1e+03) (+ (LocalVariables|GetLocalY) 2e+03) (LocalVariables|GetLargeTemperatureScale) (LocalVariables|GetSmallTemperatureScale)))
  (LocalVariables|SetSmallColdNoise _smallnoiseoutput)
  (LocalVariables|SetLargeColdNoise _largenoiseoutput)
  (bind (_smallnoiseoutput_2 _largenoiseoutput_2) (CallFunction|FGetTemperatureNoiseatCoordinate (+ (LocalVariables|GetLocalX) 1e+03) (+ (LocalVariables|GetLocalY) 2e+03) (LocalVariables|GetLargeTemperatureScale) (LocalVariables|GetSmallTemperatureScale)))
  (LocalVariables|SetSmallTemperateNoise _smallnoiseoutput_2)
  (LocalVariables|SetLargeTemperateNoise _largenoiseoutput_2)
  (bind (_smallnoiseoutput_3 _largenoiseoutput_3) (CallFunction|FGetTemperatureNoiseatCoordinate (+ (LocalVariables|GetLocalX) 1e+03) (+ (LocalVariables|GetLocalY) 2e+03) (LocalVariables|GetLargeTemperatureScale) (LocalVariables|GetSmallTemperatureScale)))
  (LocalVariables|SetSmallHotNoise _smallnoiseoutput_3)
  (LocalVariables|SetLargeHotNoise _largenoiseoutput_3)
  (LocalVariables|SetHighest (.MaxValue (Math|Float|MaxOfFloatArray (Utilities|Array|MakeArray (LocalVariables|GetLargeHotNoise) (LocalVariables|GetLargeTemperateNoise) (LocalVariables|GetLargeColdNoise)))))
  (bind _output_get (LocalVariables|SetSecondHighest (Utilities|Operators|Subtract (+ (LocalVariables|GetLargeHotNoise) (LocalVariables|GetLargeTemperateNoise) (LocalVariables|GetLargeColdNoise)) (.MinValue (Math|Float|MinOfFloatArray (Utilities|Array|MakeArray (LocalVariables|GetLargeHotNoise) (LocalVariables|GetLargeTemperateNoise) (LocalVariables|GetLargeColdNoise)))) (LocalVariables|GetHighest))))
  (LocalVariables|SetBorderMask (- 1.0 (- (LocalVariables|GetHighest) _output_get)))
  (LocalVariables|SetFinalColdNoise (+ (LocalVariables|GetLargeColdNoise) (* (LocalVariables|GetSmallColdNoise) (LocalVariables|GetBorderMask) 0.1)))
  (LocalVariables|SetFinalTemperateNoise (+ (LocalVariables|GetLargeTemperateNoise) (* (LocalVariables|GetSmallTemperateNoise) (LocalVariables|GetBorderMask) 0.1)))
  (LocalVariables|SetFinalHotNoise (+ (LocalVariables|GetLargeHotNoise) (* (LocalVariables|GetSmallHotNoise) (LocalVariables|GetBorderMask) 0.1)))
  (if (and (> (LocalVariables|GetFinalColdNoise) (LocalVariables|GetFinalTemperateNoise)) (> (LocalVariables|GetFinalColdNoise) (LocalVariables|GetFinalHotNoise)))
    (return "NewEnumerator2")
    (elif (and (> (LocalVariables|GetFinalTemperateNoise) (LocalVariables|GetFinalColdNoise)) (> (LocalVariables|GetFinalTemperateNoise) (LocalVariables|GetFinalHotNoise)))
      (return "NewEnumerator1")
      (else
        (return "NewEnumerator0")))))

(fn FGetTemperatureNoiseatCoordinate
  (params (X :type Float%20%28double-precision%29) (Y :type Float%20%28double-precision%29) (LargeScale :type Float%20%28double-precision%29) (SmallScale :type Float%20%28double-precision%29))
  (LocalVariables|SetLocalX X)
  (LocalVariables|SetLocalY Y)
  (LocalVariables|SetLocalLargeScale LargeScale)
  (LocalVariables|SetLocalSmallScale SmallScale)
  (bind _returnvalue (Class|NoiseBlueprintLibrary|GetPerlinNoise2D (Math|Vector2D|MakeVector2D (/ (LocalVariables|GetLocalX) (LocalVariables|GetLocalLargeScale)) (/ (LocalVariables|GetLocalY) (LocalVariables|GetLocalLargeScale)))))
  (LocalVariables|SetLargeNoise _returnvalue)
  (bind _returnvalue_2 (Class|NoiseBlueprintLibrary|GetPerlinNoise2D (Math|Vector2D|MakeVector2D (/ (LocalVariables|GetLocalX) (LocalVariables|GetLocalSmallScale)) (/ (LocalVariables|GetLocalY) (LocalVariables|GetLocalSmallScale)))))
  (bind _output_get (LocalVariables|SetSmallNoise _returnvalue_2))
  (return _output_get (LocalVariables|GetLargeNoise)))