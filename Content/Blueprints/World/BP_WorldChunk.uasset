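; World chunk that procedurally generates a square grid of instanced mesh tiles from its chunk coordinates.
; Layered Perlin noise picks land or sea, while competing offset noise fields pick temperature and moisture; together these define the biome.
; Only Plains gets a terrain subtype, rolled from a stream seeded by tile coordinates and WorldSeed.
; WorldDebugView selects each tile's color, written to per-instance custom data as RGB.
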(fn ConstructionScript)

(fn FGenerateChunk
  (bind _chunksize (Variables|Default|GetChunkSize))
  (bind _tilesize (Variables|Default|GetTileSize))
  (bind _returnvalue (- _chunksize 1))
  (Components|InstancedStaticMesh|ClearInstances (Variables|Default|GetISM_Tiles))
  (for _index (range 0 _returnvalue)
    (LocalVariables|SetLocalTileY _index)
    (for _index_2 (range 0 _returnvalue)
      (bind _output_get (LocalVariables|SetLocalTileX _index_2))
      (LocalVariables|SetWorldTileX (+ _output_get (* (Variables|Default|GetChunkCoordinateX) (Variables|Default|GetChunkSize))))
      (LocalVariables|SetWorldTileY (+ (LocalVariables|GetLocalTileY) (* (Variables|Default|GetChunkCoordinateY) (Variables|Default|GetChunkSize))))
      (bind _regiontype (CallFunction|FGetRegionTypeatCoordinate (LocalVariables|GetWorldTileX) (LocalVariables|GetWorldTileY)))
      (LocalVariables|SetCurrentRegionType _regiontype)
      (bind _temperaturetype (CallFunction|FGetTemperatureTypeatCoordinate (LocalVariables|GetWorldTileX) (LocalVariables|GetWorldTileY)))
      (LocalVariables|SetCurrentTemperatureType _temperaturetype)
      (bind _moisturetype (CallFunction|FGetMoistureTypeatCoordinate (LocalVariables|GetWorldTileX) (LocalVariables|GetWorldTileY)))
      (LocalVariables|SetCurrentMoistureType _moisturetype)
      (bind _biometype (CallFunction|FGetBiomeTypeatCoordinate (LocalVariables|GetCurrentRegionType) (LocalVariables|GetCurrentTemperatureType) (LocalVariables|GetCurrentMoistureType)))
      (bind _output_get_2 (LocalVariables|SetCurrentBiomeType _biometype))
      (bind _baseterraintype (CallFunction|FGetBaseTerrainTypeatCoordinate _output_get_2 (LocalVariables|GetWorldTileX) (LocalVariables|GetWorldTileY)))
      (bind _regioncolor (CallFunction|FGetRegionColor (LocalVariables|GetCurrentRegionType) (LocalVariables|GetCurrentTemperatureType) (LocalVariables|GetCurrentMoistureType) _baseterraintype))
      (LocalVariables|SetCurrentRegionColor _regioncolor)
      (bind _returnvalue_2 (Components|InstancedStaticMesh|AddInstance (Variables|Default|GetISM_Tiles) (Math|Transform|MakeTransform (Math|Vector|MakeVector (* (LocalVariables|GetLocalTileX) _tilesize) (* _tilesize (LocalVariables|GetLocalTileY)) 0.0) "0, 0, 0" "1.000000,1.000000,1.000000") false))
      (LocalVariables|SetInstanceIndex _returnvalue_2)
      (Components|InstancedStaticMesh|SetCustomDataValue (Variables|Default|GetISM_Tiles) (LocalVariables|GetInstanceIndex) 0 (.r (LocalVariables|GetCurrentRegionColor)) false)
      (Components|InstancedStaticMesh|SetCustomDataValue (Variables|Default|GetISM_Tiles) (LocalVariables|GetInstanceIndex) 1 (.g (LocalVariables|GetCurrentRegionColor)) false)
      (Components|InstancedStaticMesh|SetCustomDataValue (Variables|Default|GetISM_Tiles) (LocalVariables|GetInstanceIndex) 2 (.b (LocalVariables|GetCurrentRegionColor)) false))))

(fn FGetRegionTypeatCoordinate
  (params (X :type Integer) (Y :type Integer))
  (bind (_noisevalue _hugenoiseoutput) (CallFunction|FGetRegionNoiseatCoordinate X Y))
  (if (<= _noisevalue (+ (Variables|Default|GetLandThreshold) (* _hugenoiseoutput (Variables|Default|GetHugeRegionStrength))))
    (return "NewEnumerator1")
    (else
      (return "NewEnumerator0"))))

(fn FGetRegionNoiseatCoordinate
  (params (X :type Integer) (Y :type Integer))
  (bind _largeregionscaledivisor (Variables|Default|GetLargeRegionScaleDivisor))
  (bind _smallregionscaledivisor (Variables|Default|GetSmallRegionScaleDivisor))
  (bind _mediumregionscaledivisor (Variables|Default|GetMediumRegionScaleDivisor))
  (bind _hugeregionscaledivisor (Variables|Default|GetHugeRegionScaleDivisor))
  (LocalVariables|SetLocalX (Math|Conversions|ToFloat(Integer) X))
  (LocalVariables|SetLocalY (Math|Conversions|ToFloat(Integer) Y))
  (bind _returnvalue (Class|NoiseBlueprintLibrary|GetPerlinNoise2D (Math|Vector2D|MakeVector2D (/ (LocalVariables|GetLocalX) _hugeregionscaledivisor) (/ (LocalVariables|GetLocalY) _hugeregionscaledivisor))))
  (LocalVariables|SetHugeNoise _returnvalue)
  (bind _returnvalue_2 (Class|NoiseBlueprintLibrary|GetPerlinNoise2D (Math|Vector2D|MakeVector2D (/ (LocalVariables|GetLocalX) _largeregionscaledivisor) (/ (LocalVariables|GetLocalY) _largeregionscaledivisor))))
  (LocalVariables|SetLargeNoise _returnvalue_2)
  (bind _returnvalue_3 (Class|NoiseBlueprintLibrary|GetPerlinNoise2D (Math|Vector2D|MakeVector2D (/ (LocalVariables|GetLocalX) _mediumregionscaledivisor) (/ (LocalVariables|GetLocalY) _mediumregionscaledivisor))))
  (LocalVariables|SetMediumNoise _returnvalue_3)
  (bind _returnvalue_4 (Class|NoiseBlueprintLibrary|GetPerlinNoise2D (Math|Vector2D|MakeVector2D (/ (LocalVariables|GetLocalX) _smallregionscaledivisor) (/ (LocalVariables|GetLocalY) _smallregionscaledivisor))))
  (LocalVariables|SetSmallNoise _returnvalue_4)
  (bind _returnvalue_5 (Class|NoiseBlueprintLibrary|GetPerlinNoise2D (Math|Vector2D|MakeVector2D (/ (LocalVariables|GetLocalX) 5.0) (/ (LocalVariables|GetLocalY) (Variables|Default|GetTinyRegionScaleDivisor)))))
  (LocalVariables|SetTinyNoise _returnvalue_5)
  (bind _output_get (LocalVariables|SetFinalRegionNoise (+ (* (LocalVariables|GetLargeNoise) (Variables|Default|GetLargeRegionWeight)) (* (LocalVariables|GetMediumNoise) (Variables|Default|GetMediumRegionWeight)) (* (LocalVariables|GetSmallNoise) (Variables|Default|GetSmallRegionWeight)) (* (LocalVariables|GetTinyNoise) (Variables|Default|GetTinyRegionWeight)))))
  (return _output_get (LocalVariables|GetHugeNoise)))

(fn FGetRegionColor
  (params (RegionType :type E_RegionType%20Enum :default "NewEnumerator0") (TemperatureType :type E_TemperatureType%20Enum :default "NewEnumerator0") (MoistureType :type E_MoistureType%20Enum :default "NewEnumerator0") (TerrainType :type E_TerrainType%20Enum :default "NewEnumerator0"))
  (switch Utilities|FlowControl|Switch|SwitchonE_WorldDebugView (Variables|Default|GetWorldDebugView)
    (:NewEnumerator0
      (switch Utilities|FlowControl|Switch|SwitchonE_RegionType RegionType
        (:NewEnumerator0
          (return "(R=0.000000,G=1.000000,B=0.000000,A=1.000000)"))
        (:NewEnumerator1
          (return "(R=0.000000,G=0.000000,B=1.000000,A=1.000000)"))))
    (:NewEnumerator1
      (switch Utilities|FlowControl|Switch|SwitchonE_RegionType RegionType
        (:NewEnumerator0
          (switch Utilities|FlowControl|Switch|SwitchonE_TemperatureType TemperatureType
            (:NewEnumerator0
              (return "(R=1.000000,G=0.000000,B=0.000000,A=1.000000)"))
            (:NewEnumerator1
              (return "(R=0.000000,G=1.000000,B=0.000000,A=1.000000)"))
            (:NewEnumerator2
              (return "(R=0.000000,G=0.000000,B=1.000000,A=1.000000)"))))
        (:NewEnumerator1
          (switch Utilities|FlowControl|Switch|SwitchonE_TemperatureType TemperatureType
            (:NewEnumerator0
              (return "(R=1.000000,G=0.000000,B=0.200000,A=1.000000)"))
            (:NewEnumerator1
              (return "(R=0.000000,G=1.000000,B=0.200000,A=1.000000)"))
            (:NewEnumerator2
              (return "(R=0.100000,G=0.100000,B=1.000000,A=1.000000)"))))))
    (:NewEnumerator2
      (switch Utilities|FlowControl|Switch|SwitchonE_RegionType RegionType
        (:NewEnumerator0
          (switch Utilities|FlowControl|Switch|SwitchonE_MoistureType MoistureType
            (:NewEnumerator0
              (return "(R=1.000000,G=0.000000,B=0.000000,A=1.000000)"))
            (:NewEnumerator1
              (return "(R=0.000000,G=0.000000,B=1.000000,A=1.000000)"))))
        (:NewEnumerator1
          (switch Utilities|FlowControl|Switch|SwitchonE_MoistureType MoistureType
            (:NewEnumerator0
              (return "(R=1.000000,G=0.000000,B=0.200000,A=1.000000)"))
            (:NewEnumerator1
              (return "(R=0.100000,G=0.100000,B=1.000000,A=1.000000)"))))))
    (:NewEnumerator3
      (switch Utilities|FlowControl|Switch|SwitchonE_RegionType RegionType
        (:NewEnumerator0
          (switch Utilities|FlowControl|Switch|SwitchonE_TemperatureType TemperatureType
            (:NewEnumerator0
              (switch Utilities|FlowControl|Switch|SwitchonE_MoistureType MoistureType
                (:NewEnumerator0
                  (return "(R=1.000000,G=0.000000,B=0.000000,A=1.000000)"))
                (:NewEnumerator1
                  (return "(R=1.000000,G=0.500000,B=0.000000,A=1.000000)"))))
            (:NewEnumerator1
              (switch Utilities|FlowControl|Switch|SwitchonE_MoistureType MoistureType
                (:NewEnumerator0
                  (return "(R=0.250000,G=1.000000,B=0.000000,A=1.000000)"))
                (:NewEnumerator1
                  (return "(R=0.000000,G=1.000000,B=0.000000,A=1.000000)"))))
            (:NewEnumerator2
              (switch Utilities|FlowControl|Switch|SwitchonE_MoistureType MoistureType
                (:NewEnumerator0
                  (return "(R=0.000000,G=0.500000,B=1.000000,A=1.000000)"))
                (:NewEnumerator1
                  (return "(R=0.000000,G=0.000000,B=1.000000,A=1.000000)"))))))
        (:NewEnumerator1
          (switch Utilities|FlowControl|Switch|SwitchonE_TemperatureType TemperatureType
            (:NewEnumerator0
              (switch Utilities|FlowControl|Switch|SwitchonE_MoistureType MoistureType
                (:NewEnumerator0
                  (return "(R=1.000000,G=0.000000,B=0.250000,A=1.000000)"))
                (:NewEnumerator1
                  (return "(R=1.000000,G=0.500000,B=0.250000,A=1.000000)"))))
            (:NewEnumerator1
              (switch Utilities|FlowControl|Switch|SwitchonE_MoistureType MoistureType
                (:NewEnumerator0
                  (return "(R=0.250000,G=1.000000,B=0.250000,A=1.000000)"))
                (:NewEnumerator1
                  (return "(R=0.000000,G=1.000000,B=0.250000,A=1.000000)"))))
            (:NewEnumerator2
              (switch Utilities|FlowControl|Switch|SwitchonE_MoistureType MoistureType
                (:NewEnumerator0
                  (return "(R=0.100000,G=0.600000,B=1.000000,A=1.000000)"))
                (:NewEnumerator1
                  (return "(R=0.100000,G=0.100000,B=1.000000,A=1.000000)"))))))))
    (:NewEnumerator4
      (switch Utilities|FlowControl|Switch|SwitchonE_RegionType RegionType
        (:NewEnumerator0
          (switch Utilities|FlowControl|Switch|SwitchonE_TemperatureType TemperatureType
            (:NewEnumerator0
              (switch Utilities|FlowControl|Switch|SwitchonE_MoistureType MoistureType
                (:NewEnumerator0
                  (return "(R=0.806952,G=0.584079,B=0.187821,A=1.000000)"))
                (:NewEnumerator1
                  (return "(R=0.015996,G=0.258183,B=0.015996,A=1.000000)"))))
            (:NewEnumerator1
              (switch Utilities|FlowControl|Switch|SwitchonE_MoistureType MoistureType
                (:NewEnumerator0
                  (return "(R=0.201556,G=0.508881,B=0.064803,A=1.000000)"))
                (:NewEnumerator1
                  (return "(R=0.023153,G=0.107023,B=0.019382,A=1.000000)"))))
            (:NewEnumerator2
              (switch Utilities|FlowControl|Switch|SwitchonE_MoistureType MoistureType
                (:NewEnumerator0
                  (return "(R=0.491021,G=0.564712,B=0.584079,A=1.000000)"))
                (:NewEnumerator1
                  (return "(R=0.061246,G=0.177888,B=0.111932,A=1.000000)"))))))
        (:NewEnumerator1
          (switch Utilities|FlowControl|Switch|SwitchonE_TemperatureType TemperatureType
            (:NewEnumerator0
              (switch Utilities|FlowControl|Switch|SwitchonE_MoistureType MoistureType
                (:NewEnumerator0
                  (return "(R=0.042311,G=0.025187,B=0.078187,A=1.000000)"))
                (:NewEnumerator1
                  (return "(R=0.000535,G=0.677461,B=0.822917,A=1.000000)"))))
            (:NewEnumerator1
              (switch Utilities|FlowControl|Switch|SwitchonE_MoistureType MoistureType
                (:NewEnumerator0
                  (return "(R=0.014444,G=0.219526,B=0.401978,A=1.000000)"))
                (:NewEnumerator1
                  (return "(R=0.019382,G=0.084376,B=0.201556,A=1.000000)"))))
            (:NewEnumerator2
              (switch Utilities|FlowControl|Switch|SwitchonE_MoistureType MoistureType
                (:NewEnumerator0
                  (return "(R=0.562826,G=0.890658,B=0.947917,A=1.000000)"))
                (:NewEnumerator1
                  (return "(R=0.252104,G=1.000000,B=0.654347,A=1.000000)"))))))))
    (:NewEnumerator6
      (switch Utilities|FlowControl|Switch|SwitchonE_RegionType RegionType
        (:NewEnumerator0
          (switch Utilities|FlowControl|Switch|SwitchonE_TemperatureType TemperatureType
            (:NewEnumerator0
              (switch Utilities|FlowControl|Switch|SwitchonE_MoistureType MoistureType
                (:NewEnumerator0
                  (return "(R=0.806952,G=0.584079,B=0.187821,A=1.000000)"))
                (:NewEnumerator1
                  (return "(R=0.015996,G=0.258183,B=0.015996,A=1.000000)"))))
            (:NewEnumerator1
              (switch Utilities|FlowControl|Switch|SwitchonE_MoistureType MoistureType
                (:NewEnumerator0
                  (switch Utilities|FlowControl|Switch|SwitchonE_TerrainType TerrainType
                    (:NewEnumerator0
                      (return "(R=0.328049,G=0.508881,B=0.241045,A=1.000000)"))
                    (:NewEnumerator1
                      (return "(R=0.201556,G=0.508881,B=0.064803,A=1.000000)"))
                    (:NewEnumerator2
                      (return "(R=0.073167,G=0.208333,B=0.013021,A=1.000000)"))))
                (:NewEnumerator1
                  (return "(R=0.023153,G=0.107023,B=0.019382,A=1.000000)"))))
            (:NewEnumerator2
              (switch Utilities|FlowControl|Switch|SwitchonE_MoistureType MoistureType
                (:NewEnumerator0
                  (return "(R=0.491021,G=0.564712,B=0.584079,A=1.000000)"))
                (:NewEnumerator1
                  (return "(R=0.061246,G=0.177888,B=0.111932,A=1.000000)"))))))
        (:NewEnumerator1
          (switch Utilities|FlowControl|Switch|SwitchonE_TemperatureType TemperatureType
            (:NewEnumerator0
              (switch Utilities|FlowControl|Switch|SwitchonE_MoistureType MoistureType
                (:NewEnumerator0
                  (return "(R=0.042311,G=0.025187,B=0.078187,A=1.000000)"))
                (:NewEnumerator1
                  (return "(R=0.000535,G=0.677461,B=0.822917,A=1.000000)"))))
            (:NewEnumerator1
              (switch Utilities|FlowControl|Switch|SwitchonE_MoistureType MoistureType
                (:NewEnumerator0
                  (return "(R=0.014444,G=0.219526,B=0.401978,A=1.000000)"))
                (:NewEnumerator1
                  (return "(R=0.019382,G=0.084376,B=0.201556,A=1.000000)"))))
            (:NewEnumerator2
              (switch Utilities|FlowControl|Switch|SwitchonE_MoistureType MoistureType
                (:NewEnumerator0
                  (return "(R=0.562826,G=0.890658,B=0.947917,A=1.000000)"))
                (:NewEnumerator1
                  (return "(R=0.252104,G=1.000000,B=0.654347,A=1.000000)"))))))))))

(fn FGetTemperatureTypeatCoordinate
  (params (X :type Integer) (Y :type Integer))
  (LocalVariables|SetLocalX (Math|Conversions|ToFloat(Integer) X))
  (LocalVariables|SetLocalY (Math|Conversions|ToFloat(Integer) Y))
  (bind (_smallnoiseoutput _largenoiseoutput) (CallFunction|FGetDoubleNoiseatCoordinate (+ (LocalVariables|GetLocalX) 1e+03) (+ (LocalVariables|GetLocalY) 2e+03) (LocalVariables|GetLargeTemperatureScale) (LocalVariables|GetSmallTemperatureScale)))
  (LocalVariables|SetSmallColdNoise _smallnoiseoutput)
  (LocalVariables|SetLargeColdNoise _largenoiseoutput)
  (bind (_smallnoiseoutput_2 _largenoiseoutput_2) (CallFunction|FGetDoubleNoiseatCoordinate (+ (LocalVariables|GetLocalX) 1e+04) (+ (LocalVariables|GetLocalY) 2e+04) (LocalVariables|GetLargeTemperatureScale) (LocalVariables|GetSmallTemperatureScale)))
  (LocalVariables|SetSmallTemperateNoise _smallnoiseoutput_2)
  (LocalVariables|SetLargeTemperateNoise _largenoiseoutput_2)
  (bind (_smallnoiseoutput_3 _largenoiseoutput_3) (CallFunction|FGetDoubleNoiseatCoordinate (+ (LocalVariables|GetLocalX) 3e+04) (+ (LocalVariables|GetLocalY) 4e+04) (LocalVariables|GetLargeTemperatureScale) (LocalVariables|GetSmallTemperatureScale)))
  (LocalVariables|SetSmallHotNoise _smallnoiseoutput_3)
  (LocalVariables|SetLargeHotNoise _largenoiseoutput_3)
  (LocalVariables|SetFinalColdNoise (+ (LocalVariables|GetLargeColdNoise) (* (LocalVariables|GetSmallColdNoise) 0.1)))
  (LocalVariables|SetFinalTemperateNoise (+ (LocalVariables|GetLargeTemperateNoise) (* (LocalVariables|GetSmallTemperateNoise) 0.1)))
  (LocalVariables|SetFinalHotNoise (+ (LocalVariables|GetLargeHotNoise) (* (LocalVariables|GetSmallHotNoise) 0.1)))
  (if (and (> (LocalVariables|GetFinalColdNoise) (LocalVariables|GetFinalTemperateNoise)) (> (LocalVariables|GetFinalColdNoise) (LocalVariables|GetFinalHotNoise)))
    (return "NewEnumerator2")
    (elif (and (> (LocalVariables|GetFinalTemperateNoise) (LocalVariables|GetFinalColdNoise)) (> (LocalVariables|GetFinalTemperateNoise) (LocalVariables|GetFinalHotNoise)))
      (return "NewEnumerator1")
      (else
        (return "NewEnumerator0")))))

(fn FGetSingleNoiseatCoordinate
  (params (X :type Float%20%28double-precision%29) (Y :type Float%20%28double-precision%29) (Scale :type Float%20%28double-precision%29))
  (LocalVariables|SetLocalX X)
  (LocalVariables|SetLocalY Y)
  (LocalVariables|SetLocalScale Scale)
  (bind _returnvalue (Class|NoiseBlueprintLibrary|GetPerlinNoise2D (Math|Vector2D|MakeVector2D (/ (LocalVariables|GetLocalX) (LocalVariables|GetLocalScale)) (/ (LocalVariables|GetLocalY) (LocalVariables|GetLocalScale)))))
  (bind _output_get (LocalVariables|SetLocalNoise _returnvalue))
  (return _output_get))

(fn FGetDoubleNoiseatCoordinate
  (params (X :type Float%20%28double-precision%29) (Y :type Float%20%28double-precision%29) (LargeScale :type Float%20%28double-precision%29) (SmallScale :type Float%20%28double-precision%29))
  (LocalVariables|SetLocalX X)
  (LocalVariables|SetLocalY Y)
  (LocalVariables|SetLocalLargeScale LargeScale)
  (LocalVariables|SetLocalSmallScale SmallScale)
  (bind _returnvalue (Class|NoiseBlueprintLibrary|GetPerlinNoise2D (Math|Vector2D|MakeVector2D (/ (LocalVariables|GetLocalX) (LocalVariables|GetLocalLargeScale)) (/ (LocalVariables|GetLocalY) (LocalVariables|GetLocalLargeScale)))))
  (LocalVariables|SetLargeNoise _returnvalue)
  (bind _returnvalue_2 (Class|NoiseBlueprintLibrary|GetPerlinNoise2D (Math|Vector2D|MakeVector2D (/ (LocalVariables|GetLocalX) (LocalVariables|GetLocalSmallScale)) (/ (LocalVariables|GetLocalY) (LocalVariables|GetLocalSmallScale)))))
  (bind _output_get (LocalVariables|SetSmallNoise _returnvalue_2))
  (return _output_get (LocalVariables|GetLargeNoise)))

(fn FGetMoistureTypeatCoordinate
  (params (X :type Integer) (Y :type Integer))
  (LocalVariables|SetLocalX (Math|Conversions|ToFloat(Integer) X))
  (LocalVariables|SetLocalY (Math|Conversions|ToFloat(Integer) Y))
  (bind (_smallnoiseoutput _largenoiseoutput) (CallFunction|FGetDoubleNoiseatCoordinate (+ (LocalVariables|GetLocalX) -2e+03) (+ (LocalVariables|GetLocalY) -4e+03) (LocalVariables|GetLargeMoistureScale) (LocalVariables|GetSmallMoistureScale)))
  (LocalVariables|SetSmallDryNoise _smallnoiseoutput)
  (LocalVariables|SetLargeDryNoise _largenoiseoutput)
  (bind (_smallnoiseoutput_2 _largenoiseoutput_2) (CallFunction|FGetDoubleNoiseatCoordinate (+ (LocalVariables|GetLocalX) -1e+04) (+ (LocalVariables|GetLocalY) -2e+04) (LocalVariables|GetLargeMoistureScale) (LocalVariables|GetSmallMoistureScale)))
  (LocalVariables|SetSmallWetNoise _smallnoiseoutput_2)
  (LocalVariables|SetLargeWetNoise _largenoiseoutput_2)
  (LocalVariables|SetFinalDryNoise (+ (LocalVariables|GetLargeDryNoise) (* (LocalVariables|GetSmallDryNoise) 0.1)))
  (bind _output_get (LocalVariables|SetFinalWetNoise (+ (LocalVariables|GetLargeWetNoise) (* (LocalVariables|GetSmallWetNoise) 0.1))))
  (if (< _output_get (LocalVariables|GetFinalDryNoise))
    (return "NewEnumerator0")
    (else
      (return "NewEnumerator1"))))

(fn FGetBiomeTypeatCoordinate
  (params (RegionType :type E_RegionType%20Enum :default "NewEnumerator0") (TemperatureType :type E_TemperatureType%20Enum :default "NewEnumerator0") (MoistureType :type E_MoistureType%20Enum :default "NewEnumerator0"))
  (LocalVariables|SetCurrentRegionType RegionType)
  (LocalVariables|SetCurrentTemperatureType TemperatureType)
  (LocalVariables|SetCurrentMoistureType MoistureType)
  (switch Utilities|FlowControl|Switch|SwitchonE_RegionType (LocalVariables|GetCurrentRegionType)
    (:NewEnumerator0
      (switch Utilities|FlowControl|Switch|SwitchonE_MoistureType (LocalVariables|GetCurrentMoistureType)
        (:NewEnumerator0
          (switch Utilities|FlowControl|Switch|SwitchonE_TemperatureType (LocalVariables|GetCurrentTemperatureType)
            (:NewEnumerator0
              (return "NewEnumerator0"))
            (:NewEnumerator1
              (return "NewEnumerator2"))
            (:NewEnumerator2
              (return "NewEnumerator4"))))
        (:NewEnumerator1
          (switch Utilities|FlowControl|Switch|SwitchonE_TemperatureType (LocalVariables|GetCurrentTemperatureType)
            (:NewEnumerator0
              (return "NewEnumerator1"))
            (:NewEnumerator1
              (return "NewEnumerator3"))
            (:NewEnumerator2
              (return "NewEnumerator5"))))))
    (:NewEnumerator1
      (switch Utilities|FlowControl|Switch|SwitchonE_MoistureType (LocalVariables|GetCurrentMoistureType)
        (:NewEnumerator0
          (switch Utilities|FlowControl|Switch|SwitchonE_TemperatureType (LocalVariables|GetCurrentTemperatureType)
            (:NewEnumerator0
              (return "NewEnumerator7"))
            (:NewEnumerator1
              (return "NewEnumerator8"))
            (:NewEnumerator2
              (return "NewEnumerator11"))))
        (:NewEnumerator1
          (switch Utilities|FlowControl|Switch|SwitchonE_TemperatureType (LocalVariables|GetCurrentTemperatureType)
            (:NewEnumerator0
              (return "NewEnumerator6"))
            (:NewEnumerator1
              (return "NewEnumerator9"))
            (:NewEnumerator2
              (return "NewEnumerator10"))))))))

(fn FGetBaseTerrainTypeatCoordinate
  (params (BiomeType :type E_BiomeType%20Enum :default "NewEnumerator0") (X :type Integer) (Y :type Integer))
  (bind _randomstream (LocalVariables|GetRandomStream))
  (bind _returnvalue (Math|Random|RandomFloatfromStream _randomstream))
  (LocalVariables|SetCurrentBiomeType BiomeType)
  (LocalVariables|SetLocalX X)
  (LocalVariables|SetLocalY Y)
  (switch Utilities|FlowControl|Switch|SwitchonE_BiomeType (LocalVariables|GetCurrentBiomeType)
    (:NewEnumerator2
      (bind _returnvalue_2 (Class|NoiseBlueprintLibrary|HashCombineFastInt (LocalVariables|GetLocalX) (LocalVariables|GetLocalY)))
      (bind _returnvalue_3 (Class|NoiseBlueprintLibrary|HashCombineFastInt _returnvalue_2 (Variables|Default|GetWorldSeed)))
      (bind _output_get (LocalVariables|SetTileSeed _returnvalue_3))
      (Math|Random|SetRandomStreamSeed _randomstream _output_get)
      (if (< _returnvalue 0.5)
        (return "NewEnumerator1")
        (elif (and (>= _returnvalue 0.5) (< _returnvalue 0.6))
          (return "NewEnumerator2")
          (else
            (return "NewEnumerator0")))))))